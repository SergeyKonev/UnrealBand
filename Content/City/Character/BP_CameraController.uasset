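; Character-based camera controller in the City content that moves, orbits, pitches and zooms a spring arm view.
; Movement follows control yaw only, orbit adds controller yaw, and pitch rotates the spring arm within clamped angles.
; Zoom changes arm length within limits, then rescales max walk speed by arm length relative to minimum zoom, so movement is faster when zoomed out.
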(event `self.ReceiveBeginPlay`
  (set `self.InitialMovementSpeed` (`CharacterMovementComponent.MaxWalkSpeed` (`self.CharacterMovement`)))
  (`self.UpdateMovementSpeed`))

(event `CameraOrbit`
  (params (Magnitude :type "Float (double-precision)"))
  (`self.AddControllerYawInput` (* Magnitude (`self.OrbitSpeed`))))

(event `CameraPitch`
  (params (Magnitude :type "Float (double-precision)"))
  (bind (_returnvalue_roll _returnvalue_pitch _returnvalue_yaw) (`KismetMathLibrary.BreakRotator` (`SceneComponent.K2_GetComponentRotation` (`self.SpringArm`))))
  (`SceneComponent.K2_SetWorldRotation` (`self.SpringArm`) (`KismetMathLibrary.MakeRotator` _returnvalue_roll (`KismetMathLibrary.ClampAngle` (+ (* (`self.OrbitSpeed`) Magnitude) _returnvalue_pitch) (`self.CameraMinClamp`) (`self.CameraMaxClamp`)) _returnvalue_yaw) false false))

(event `MoveForward`
  (params (Magnitude :type "Float (double-precision)"))
  (`self.AddMovementInput` (`KismetMathLibrary.GetForwardVector` (`KismetMathLibrary.MakeRotator` 0.0 0.0 (.yaw (`self.GetControlRotation`)))) Magnitude))

(event `LeftRightStrafe`
  (params (Magnitude :type "Float (double-precision)"))
  (`self.AddMovementInput` (`KismetMathLibrary.GetRightVector` (`KismetMathLibrary.MakeRotator` 0.0 0.0 (.yaw (`self.GetControlRotation`)))) Magnitude))

(event `CameraZoom`
  (params (Magnitude :type "Float (double-precision)"))
  (bind _springarm (`self.SpringArm`))
  (set `SpringArmComponent.TargetArmLength` (`KismetMathLibrary.FClamp` (+ (* Magnitude (`self.ZoomSpeedIn`)) (`SpringArmComponent.TargetArmLength` _springarm)) (`self.ZoomMin`) (`self.ZoomMax`)) _springarm)
  (`self.UpdateMovementSpeed`))

(fn `UpdateMovementSpeed`
  (set `CharacterMovementComponent.MaxWalkSpeed` (* (`self.InitialMovementSpeed`) (/ (`SpringArmComponent.TargetArmLength` (`self.SpringArm`)) (`self.ZoomMin`))) (`self.CharacterMovement`)))

(fn `UserConstructionScript`)