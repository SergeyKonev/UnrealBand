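; BP_CityPause is a Blueprint that toggles the city pause menu, enabling its own input on BeginPlay.
; P creates a UI_CityPause widget, pauses the game, shows the cursor and switches to game-and-UI input focused on the widget.
; U removes top-level UI_CityPause widgets by class lookup, unpauses and restores game-only input, leaving the cursor visible.
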(event `ShowCityPauseMenu`
  (bind _returnvalue (`GameplayStatics.GetPlayerController` 0))
  (bind _returnvalue_2 (`|CreateWidget` "/Game/City/UI_CityPause.UI_CityPause_C" _returnvalue))
  (set `self.Pause` _returnvalue_2)
  (`UserWidget.AddToViewport` (`self.Pause`) 0)
  (`WidgetBlueprintLibrary.SetInputMode_GameAndUIEx` _returnvalue (`self.Pause`))
  (`GameplayStatics.SetGamePaused` true)
  (set `PlayerController.bShowMouseCursor` true _returnvalue))

(event `ResumeCityPauseMenu`
  (bind _returnvalue (`GameplayStatics.GetPlayerController` 0))
  (bind _foundwidgets (`WidgetBlueprintLibrary.GetAllWidgetsOfClass` "/Game/City/UI_CityPause.UI_CityPause_C"))
  (`Widget.RemoveFromParent` _foundwidgets)
  (`GameplayStatics.SetGamePaused` false)
  (`WidgetBlueprintLibrary.SetInputMode_GameOnly` _returnvalue)
  (set `PlayerController.bShowMouseCursor` true _returnvalue))

(event `Key|P`
  (params (Key :type "Key Structure"))
  (:`Pressed`
    (`self.ShowCityPauseMenu`)))

(event `Key|U`
  (params (Key :type "Key Structure"))
  (:`Pressed`
    (`self.ResumeCityPauseMenu`)))

(event `self.ReceiveBeginPlay`
  (`self.EnableInput` (`GameplayStatics.GetPlayerController` 0)))

(fn `UserConstructionScript`)