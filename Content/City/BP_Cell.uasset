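; City grid cell actor that spawns a building on itself when clicked.
; On BeginPlay it caches the GI_Undeads game instance and tags itself with its "X:Y" coordinates.
; A cube click calls BuildContent to spawn the BldPrms class, but MyBld is set to None, so repeat clicks spawn again.
; Logic that records the building in the save game is present but unconnected.
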(event `self.ReceiveBeginPlay`
  ;[1 0.8287 0.2811] Enable restoring this cell's state/building from save file
  (`|ExecutionSequence`
    (:`then_0`
      (bind _asgi_undeads (cast `/Game/City/GI_Undeads` (`GameplayStatics.GetGameInstance`)))
      (set `self.My Game Instance` _asgi_undeads))
    (:`then_1`
      (`KismetArrayLibrary.Array_Add` (`self.Tags`) (`KismetStringLibrary.Conv_StringToName` (`KismetStringLibrary.Concat_StrStr` (`KismetStringLibrary.Conv_IntToString` (`self.X`)) ":" (`KismetStringLibrary.Conv_IntToString` (`self.Y`))))))))

(event `self.Cube.OnClicked`
  (params (TouchedComponent :type "PrimitiveComponent Object Reference") (ButtonPressed :type "Key Structure"))
  ;[0.4573 0.7705 1] Place the selected card's building in this cell on click
  (`/Engine/EditorBlueprintResources/StandardMacros.IsValid` (`self.My Bld`)
    (:`Is Not Valid`
      (`self.BuildContent`))))

(fn `BuildContent`
  (`|SpawnActorFromClass` (`.Class_15_6732096146F94E5DC1C786A92F24CF16` (break `/Game/City/SK_Building` (`self.Bld Prms`))) (`self.GetTransform`) "Undefined" "OverrideRootScale" null null)
  (set `self.My Bld` null))

(fn `UserConstructionScript`)