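; BP_Grid is an actor that lays out a city grid of BP_Cell actors centered on its own location.
; The construction script adds one scaled FloorTile instance sized one tile beyond GridX and GridY.
; On BeginPlay, PopulateGrid loops inclusively across both half-extents, spawns a cell at each TileSize-spaced world position, and records coordinates, location and cell reference in GridLocations.
; Cell positions ignore actor rotation and scale.
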(event `self.ReceiveBeginPlay`
  (`self.PopulateGrid`))

(fn `GetCellLocation`
  (params (X :type "Float (double-precision)") (Y :type "Float (double-precision)"))
  (returns (ReturnValue :type "Vector Structure"))
  (bind (_returnvalue_x _returnvalue_y _returnvalue_z) (`KismetMathLibrary.BreakVector` (`self.K2_GetActorLocation`)))
  (bind _tilesize (`self.TileSize`))
  (return (`KismetMathLibrary.MakeVector` (+ (* X _tilesize) _returnvalue_x) (+ (* Y _tilesize) _returnvalue_y) _returnvalue_z)))

(fn `GetCenteredCoords`
  (params (Coord :type Integer))
  (returns (CenteredCoord :type "Float (double-precision)"))
  (return (- (`KismetMathLibrary.Conv_IntToDouble` (* Coord (`self.TileSize`))) (/ (* (`self.TileSize`) (`self.GridX`)) 2))))

(fn `PopulateGrid`
  (locals (X :type Integer) (Y :type Integer))
  (bind _gridx (`self.GridX`))
  (bind _gridy (`self.GridY`))
  (`KismetArrayLibrary.Array_Clear` (`self.GridLocations`))
  (for _index (range (/ _gridx -2) (+ (/ _gridx 2) 1))
    (set `local.X` _index)
    (for _index_2 (range (/ _gridy -2) (+ (/ _gridy 2) 1))
      (set `local.Y` _index_2)
      (bind _returnvalue (`self.GetCellLocation` (`KismetMathLibrary.Conv_IntToDouble` (`local.X`)) (`KismetMathLibrary.Conv_IntToDouble` (`local.Y`))))
      (bind _returnvalue_2 (`|SpawnActorFromClass` "/Game/City/BP_Cell.BP_Cell_C" (`KismetMathLibrary.MakeTransform` _returnvalue) "Undefined" "OverrideRootScale" null null))
      (`KismetArrayLibrary.Array_Add` (`self.GridLocations`) (make `/Game/City/MapContent/SK_CellInfo` (`local.X`) (`local.Y`) "NewEnumerator0" _returnvalue _returnvalue_2)))))

(fn `UserConstructionScript`
  (`InstancedStaticMeshComponent.AddInstance` (`self.FloorTile`) (`KismetMathLibrary.MakeTransform` (0.0 0.0 0.0) (struct) (`KismetMathLibrary.MakeVector` (+ (`KismetMathLibrary.Conv_IntToDouble` (`self.GridX`)) 1.0) (+ (`KismetMathLibrary.Conv_IntToDouble` (`self.GridY`)) 1.0) 1.0)) false))