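; BP_BuildingOld is a city map building Blueprint that shows a name label when the cursor hovers over its mesh.
; On BeginPlay it casts its widget component's widget to UI_Building and sets the building name to placeholder text.
; Cursor-over events on BuildingMesh toggle the widget component's visibility, and the construction script is empty.
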(event `self.ReceiveBeginPlay`
  (bind _asui_building (cast `/Game/City/UI_Building` (`WidgetComponent.GetWidget` (`self.Widget`))))
  (`TextBlock.SetText` (`/Game/City/UI_Building.BuildingName` _asui_building) "TODO name"))

(event `self.BuildingMesh.OnBeginCursorOver`
  (params (TouchedComponent :type "PrimitiveComponent Object Reference"))
  (`SceneComponent.SetVisibility` (`self.Widget`) true false))

(event `self.BuildingMesh.OnEndCursorOver`
  (params (TouchedComponent :type "PrimitiveComponent Object Reference"))
  (`SceneComponent.SetVisibility` (`self.Widget`) false false))

(fn `UserConstructionScript`)