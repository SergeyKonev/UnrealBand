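; Building actor for the city map, with placement feedback, rotation and a hover info widget.
; On BeginPlay it creates a dynamic material for the mesh and sets a placeholder name on its UI_Building widget.
; Cursor hover on the mesh shows or hides that widget.
; Custom events toggle the material's CanBuilded parameter to signal build validity and rotate the root in 90-degree steps either way.
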(event `self.ReceiveBeginPlay`
  (bind _returnvalue (`PrimitiveComponent.CreateDynamicMaterialInstance` (`self.BuildingMesh`) 0 null "None"))
  (set `self.BuildingMaterial` _returnvalue)
  (bind _asui_building (cast `/Game/City/UI_Building` (`WidgetComponent.GetWidget` (`self.Widget`))))
  (`TextBlock.SetText` (`/Game/City/UI_Building.BuildingName` _asui_building) "TODO name"))

(event `self.BuildingMesh.OnBeginCursorOver`
  (params (TouchedComponent :type "PrimitiveComponent Object Reference"))
  (`SceneComponent.SetVisibility` (`self.Widget`) true false))

(event `self.BuildingMesh.OnEndCursorOver`
  (params (TouchedComponent :type "PrimitiveComponent Object Reference"))
  (`SceneComponent.SetVisibility` (`self.Widget`) false false))

(event `HighlightPossibilityToBuild`
  (params (CanBuild :type Boolean))
  (bind _buildingmaterial (`self.BuildingMaterial`))
  (if CanBuild
    (`MaterialInstanceDynamic.SetScalarParameterValue` _buildingmaterial "CanBuilded" 1.0)
    (else
      (`MaterialInstanceDynamic.SetScalarParameterValue` _buildingmaterial "CanBuilded" 0.0))))

(event `Rotate`
  (params (Clockwise :type Boolean))
  (bind _defaultsceneroot (`self.DefaultSceneRoot`))
  (if Clockwise
    (`SceneComponent.K2_AddLocalRotation` _defaultsceneroot (struct :`Yaw` 90.0) false false)
    (else
      (`SceneComponent.K2_AddLocalRotation` _defaultsceneroot (struct :`Yaw` -90.0) false false))))

(fn `UserConstructionScript`
  (`parent.UserConstructionScript`))