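; BP_CellContent is a map content actor for the city that lays out a rectangular floor of tiles.
; Its Construction Script loops over SizeX by SizeY and adds a FloorTile instance at each step, spaced by FloorSize.
; Instances are placed in world space from the actor's location, with fixed rotation and unit scale, so actor rotation and scale are ignored.
; The Event Graph holds no active logic.
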(fn `UserConstructionScript`
  (bind _floorsize (`self.FloorSize`))
  (for _index (range (`self.SizeX`))
    (for _index_2 (range (`self.SizeY`))
      (`InstancedStaticMeshComponent.AddInstance` (`self.FloorTile`) (`KismetMathLibrary.MakeTransform` (+ (`KismetMathLibrary.MakeVector` (`KismetMathLibrary.Conv_IntToDouble` (* _index _floorsize)) (`KismetMathLibrary.Conv_IntToDouble` (* _index_2 _floorsize))) (`self.K2_GetActorLocation`))) true))))