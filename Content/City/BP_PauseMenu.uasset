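; Actor Blueprint that toggles a pause menu through keyboard keys.
; P prints a debug message, then creates a UI_PauseMenu1 widget, pauses the game and sets Game and UI input with a visible cursor.
; U removes top-level UI_PauseMenu widgets (a different class from the one created), unpauses and restores game-only input, leaving the cursor visible.
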(event `ShowPauseMenu1`
  (bind _returnvalue (`GameplayStatics.GetPlayerController` 0))
  (bind _returnvalue_2 (`|CreateWidget` "/Game/City/UI_PauseMenu1.UI_PauseMenu1_C"))
  (set `self.pause` _returnvalue_2)
  (`UserWidget.AddToViewport` (`self.pause`) 0)
  (`WidgetBlueprintLibrary.SetInputMode_GameAndUIEx` _returnvalue (`self.pause`) "DoNotLock" false)
  (`GameplayStatics.SetGamePaused` true)
  (set `PlayerController.bShowMouseCursor` true _returnvalue))

(event `PauseMenuResume1`
  (bind _returnvalue (`GameplayStatics.GetPlayerController` 0))
  (bind _foundwidgets (`WidgetBlueprintLibrary.GetAllWidgetsOfClass` "/Game/Night/UI_PauseMenu.UI_PauseMenu_C"))
  (`Widget.RemoveFromParent` _foundwidgets)
  (`GameplayStatics.SetGamePaused` false)
  (`WidgetBlueprintLibrary.SetInputMode_GameOnly` _returnvalue)
  (set `PlayerController.bShowMouseCursor` true _returnvalue))

(event `Key|P` :paused true
  (params (Key :type "Key Structure"))
  (:`Pressed`
    (`KismetSystemLibrary.PrintText` "Hello")
    (`self.ShowPauseMenu1`)))

(event `Key|U` :paused true
  (params (Key :type "Key Structure"))
  (:`Pressed`
    (`self.PauseMenuResume1`)))

(fn `UserConstructionScript`)