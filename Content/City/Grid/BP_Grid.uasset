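; BP_Grid is an unfinished tile grid actor in the City folder, set up for drawn lines and a highlighted selected tile.
; The construction script calls CreateMaterialInstance with line and selection color and opacity, but that helper only creates a dynamic material instance without applying either input.
; Line creation, grid sizing, location-to-tile conversion, tile validation and selection are empty stubs or return default values, and the event graph is inactive.
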(fn `CreateLine`
  (params (Start :type "Vector Structure") (End :type "Vector Structure") (Thickness :type "Float (double-precision)") (Vertices :type "Array of Vector Structure") (Triangles :type "Array of Integer")))

(fn `CreateMaterialInstance`
  (params (Color :type "LinearColor Structure") (Opacity :type "Float (double-precision)"))
  (`KismetMaterialLibrary.CreateDynamicMaterialInstance` null))

(fn `GridHeight`)

(fn `GridWidth`)

(fn `LocationToTile`
  (params (Location :type "Vector Structure"))
  (returns (Row :type Integer) (Column :type Integer) (`Valid?` :type Boolean))
  (return 0 0 false))

(fn `SetSelectedTile`)

(fn `TileToGridLocation`
  (params (Row :type Integer) (Column :type Integer) (`Center?` :type Boolean))
  (returns (`Valid?` :type Boolean) (GridLocation :type "Vector2D Structure"))
  (return false (0.0 0.0)))

(fn `UserConstructionScript`
  (`self.CreateMaterialInstance` (`self.LineColor`) (`self.LineOpacity`))
  (`self.CreateMaterialInstance` (`self.SelectionColor`) (`self.SelectionOpacity`)))