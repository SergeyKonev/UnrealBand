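; BP_XP is an experience collector that pulls in BP_Experience orbs and converts them into hero XP.
; Each tick, orbs inside MagnetSphere lose gravity and receive an impulse toward CollectSphere that strengthens as they get closer.
; Orbs overlapping CollectSphere are destroyed, granting fixed XP through BPCHeroExperience on the BP_Hero nearest the world origin, rather than the collector.
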(event `self.ReceiveTick`
  (params (DeltaSeconds :type "Float (single-precision)"))
  (for _array_element (`PrimitiveComponent.GetOverlappingActors` (`self.MagnetSphere`) null)
    (bind _asbp_experience (cast `/Game/Night/BP_Experience` _array_element))
    (set `/Game/Night/BP_Experience.IsCollecting` true _asbp_experience)
    (`PrimitiveComponent.SetEnableGravity` (`/Game/Night/BP_Experience.Sphere` _asbp_experience) false)
    (`self.MagnetizeXp` _asbp_experience)))

(event `self.CollectSphere.OnComponentBeginOverlap`
  (params (OverlappedComponent :type "PrimitiveComponent Object Reference") (OtherActor :type "Actor Object Reference") (OtherComp :type "PrimitiveComponent Object Reference") (OtherBodyIndex :type Integer) (bFromSweep :type Boolean) (SweepResult :type "HitResult Structure (by ref)"))
  (bind _asbp_experience (cast `/Game/Night/BP_Experience` OtherActor))
  (`self.CollectXp` _asbp_experience))

(event `self.MagnetSphere.OnComponentBeginOverlap`
  (params (OverlappedComponent :type "PrimitiveComponent Object Reference") (OtherActor :type "Actor Object Reference") (OtherComp :type "PrimitiveComponent Object Reference") (OtherBodyIndex :type Integer) (bFromSweep :type Boolean) (SweepResult :type "HitResult Structure (by ref)")))

(fn `CollectXp`
  (params (`XP Orb` :type "/Game/Night/BP_Experience Object Reference"))
  (`self.K2_DestroyActor` `XP Orb`)
  (bind _outactors (`GameplayStatics.GetAllActorsOfClass` "/Game/Night/BP_Hero.BP_Hero_C"))
  (bind _asbp_hero (cast `/Game/Night/BP_Hero` (`.ReturnValue` (`GameplayStatics.FindNearestActor` (0.0 0.0 0.0) _outactors))))
  (`/Game/Night/BPC_HeroExperience.Add XP` (`/Game/Night/BP_Hero.BPC_HeroExperience` _asbp_hero) 25.0))

(fn `MagnetizeXp`
  (params (`XP Orb` :type "/Game/Night/BP_Experience Object Reference"))
  (bind _sphere (`/Game/Night/BP_Experience.Sphere` `XP Orb`))
  (bind _returnvalue (- (`SceneComponent.K2_GetComponentLocation` (`self.CollectSphere`)) (`self.K2_GetActorLocation` `XP Orb`)))
  (`PrimitiveComponent.AddImpulse` _sphere (* (`KismetMathLibrary.Normal` _returnvalue) (/ 50.0 (`KismetMathLibrary.MapRangeClamped` (`KismetMathLibrary.VSize` _returnvalue) 100.0 300.0 0.5 1.0))) "None" false)
  (`self.K2_SetActorLocation` `XP Orb` (`SceneComponent.K2_GetComponentLocation` _sphere) false false))

(fn `UserConstructionScript`)