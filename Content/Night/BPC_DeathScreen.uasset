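; BPC_DeathScreen is a Blueprint that displays the death screen and pauses the game.
; ShowDeathScreen creates a UI_DeathScreen widget for the first player controller, stores it and adds it to the viewport.
; It then switches input to Game and UI with the widget focused, pauses the game and shows the mouse cursor.
; Pressing the 1 key also triggers ShowDeathScreen directly.
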(event `ShowDeathScreen`
  (bind _returnvalue (`GameplayStatics.GetPlayerController` 0))
  (bind _returnvalue_2 (`|CreateWidget` "/Game/Night/UI_DeathScreen.UI_DeathScreen_C" _returnvalue))
  (set `self.DeathScreenVar` _returnvalue_2)
  (`UserWidget.AddToViewport` (`self.DeathScreenVar`) 0)
  (`WidgetBlueprintLibrary.SetInputMode_GameAndUIEx` _returnvalue (`self.DeathScreenVar`) "DoNotLock" false)
  (`GameplayStatics.SetGamePaused` true)
  (set `PlayerController.bShowMouseCursor` true _returnvalue))

(event `Key|One`
  (params (Key :type "Key Structure"))
  (:`Pressed`
    (`self.ShowDeathScreen`)))