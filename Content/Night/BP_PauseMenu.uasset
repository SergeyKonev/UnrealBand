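; BP_PauseMenu is an actor Blueprint that opens and closes the game's pause menu.
; ShowPauseMenu lazily creates and caches a UI_PauseMenu widget, adds it to the viewport, switches to UI-only input and pauses the game.
; PauseMenuResume removes top-level UI_PauseMenu widgets found by class lookup rather than the cached reference, then unpauses and restores game-only input.
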(event `ShowPauseMenu`
  (bind _returnvalue (`GameplayStatics.GetPlayerController` 0))
  ;[1 1 1] Pause
  (`/Engine/EditorBlueprintResources/StandardMacros.IsValid` (`self.PauseMenuWB`)
    (:`Is Valid`
      _)
    (:`Is Not Valid`
      (bind _returnvalue_2 (`|CreateWidget` "/Game/Night/UI_PauseMenu.UI_PauseMenu_C" _returnvalue))
      (set `self.PauseMenuWB` _returnvalue_2)))
  (`UserWidget.AddToViewport` (`self.PauseMenuWB`) 0)
  (`WidgetBlueprintLibrary.SetInputMode_UIOnlyEx` _returnvalue (`self.PauseMenuWB`) "LockInFullscreen")
  (`GameplayStatics.SetGamePaused` true))

(event `PauseMenuResume`
  (bind _foundwidgets (`WidgetBlueprintLibrary.GetAllWidgetsOfClass` "/Game/Night/UI_PauseMenu.UI_PauseMenu_C"))
  (`Widget.RemoveFromParent` _foundwidgets)
  (`GameplayStatics.SetGamePaused` false)
  (`WidgetBlueprintLibrary.SetInputMode_GameOnly` (`GameplayStatics.GetPlayerController` 0)))

(fn `UserConstructionScript`)