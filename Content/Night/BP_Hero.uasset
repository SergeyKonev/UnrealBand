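; Hero character Blueprint with sprinting, a green health bar and the in-game HUD, both set up on BeginPlay.
; Tick polls the Shift modifier and BPCSprinting to pick Run or Walk, which set movement speed and acceleration and report sprint or chill to that component.
; AddWeapon looks up a tag in DT_Weapons and adds that row's component class to the hero.
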(event `self.ReceiveBeginPlay`
  (bind _asui_damageable_bar (cast `/Game/Night/UI_Damageable_Bar` (`WidgetComponent.GetWidget` (`/Game/Night/BP_Damageable_Actor.Widget` (`/Game/Night/BPC_Damageable.Damageable Actor` (`self.BPC_Damageable`))))))
  (`ProgressBar.SetFillColorAndOpacity` (`/Game/Night/UI_Damageable_Bar.HealthBar` _asui_damageable_bar) (struct :`G` 1.0 :`B` 0.207111 :`A` 1.0))
  (bind _returnvalue (`|CreateWidget` "/Game/Night/UI_Game.UI_Game_C"))
  (`UserWidget.AddToViewport` _returnvalue 0))

(event `self.ReceiveTick`
  (params (DeltaSeconds :type "Float (single-precision)"))
  (bind _returnvalue (`/Game/Night/BPC_Sprinting.Can Sprint` (`self.BPC_Sprinting`)))
  (if (and _returnvalue (`KismetInputLibrary.ModifierKeysState_IsShiftDown` (`KismetInputLibrary.GetModifierKeysState`)))
    (`self.Run`)
    (else
      (`self.Walk`))))

(fn `Add Weapon`
  (params (Tag :type String))
  (bind _returnvalue (`|GetDataTableRow` "/Game/Night/Weapons/DT_Weapons.DT_Weapons" (`KismetStringLibrary.Conv_StringToName` Tag))
    (:`then`
      (`|AddComponentByClass` (`.Component_9_D2EA33814F4A7972245013BF8146416B` (break `/Game/Night/Weapons/SK_Weapon` _returnvalue))))))

(fn `Run`
  (set `CharacterMovementComponent.MaxAcceleration` (`self.Run Acceleration`) (`self.CharacterMovement`))
  (set `CharacterMovementComponent.MaxWalkSpeed` (`self.Run Speed`) (`self.CharacterMovement`))
  (`/Game/Night/BPC_Sprinting.On Sprint` (`self.BPC_Sprinting`) 1.0))

(fn `UserConstructionScript`)

(fn `Walk`
  (set `CharacterMovementComponent.MaxAcceleration` (`self.Walk Acceleration`) (`self.CharacterMovement`))
  (set `CharacterMovementComponent.MaxWalkSpeed` (`self.Walk Speed`) (`self.CharacterMovement`))
  (`/Game/Night/BPC_Sprinting.On Chill` (`self.BPC_Sprinting`) 0.1))