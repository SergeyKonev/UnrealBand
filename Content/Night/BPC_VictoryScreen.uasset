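; Blueprint (BPC) that displays the victory screen and halts gameplay.
; ShowVictoryScreen creates and stores a UI_VictoryScreen widget for the first player controller and adds it to the viewport.
; It then switches input to Game and UI focused on the widget, pauses the game and shows the mouse cursor.
; A hardcoded 2 key press also triggers the event directly, with no win-condition check.
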(event `ShowVictoryScreen`
  (bind _returnvalue (`|CreateWidget` "/Game/Night/UI_VictoryScreen.UI_VictoryScreen_C" (`GameplayStatics.GetPlayerController` 0)))
  (set `self.VictoryScreen` _returnvalue)
  (`UserWidget.AddToViewport` (`self.VictoryScreen`) 0)
  (`WidgetBlueprintLibrary.SetInputMode_GameAndUIEx` (`GameplayStatics.GetPlayerController` 0) (`self.VictoryScreen`) "DoNotLock" false)
  (`GameplayStatics.SetGamePaused` true)
  (set `PlayerController.bShowMouseCursor` true (`GameplayStatics.GetPlayerController` 0)))

(event `Key|Two`
  (params (Key :type "Key Structure"))
  (:`Pressed`
    (`self.ShowVictoryScreen`)))