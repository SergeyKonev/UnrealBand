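; BP_Level is a registry of where BP_LevelPart actors sit in the level.
; Its construction script gathers every BP_LevelPart and records its world location as a key in the LevelParts map through AddLevelPart.
; CheckLevelPart looks up a given location in that map to report whether a part is registered there, so the query needs no actor search.
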(fn `AddLevelPart`
  (params (NewParam :type "Vector Structure"))
  (`BlueprintMapLibrary.Map_Add` (`self.LevelParts`) NewParam true))

(fn `CheckLevelPart`
  (params (NewParam :type "Vector Structure"))
  (returns (NewParam1 :type Boolean))
  (if (`BlueprintMapLibrary.Map_Find` (`self.LevelParts`) NewParam)
    (return true)
    (else
      (return false))))

(fn `UserConstructionScript`
  (bind _outactors (`GameplayStatics.GetAllActorsOfClass` "/Game/Night/BP_LevelPart.BP_LevelPart_C"))
  (for _array_element _outactors
    (bind _returnvalue_location (`KismetMathLibrary.BreakTransform` (`self.GetTransform` _array_element)))
    (`self.AddLevelPart` _returnvalue_location)))