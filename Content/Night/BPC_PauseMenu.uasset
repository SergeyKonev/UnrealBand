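; BPC_PauseMenu is a Blueprint that opens and closes the game's pause menu, bound to the P and U keys.
; P creates a new UI_PauseMenu widget, adds it to the viewport, pauses the game and switches to game-and-UI input with a visible cursor.
; U removes top-level pause menu widgets found by class, unpauses and restores game-only input, but leaves the cursor flag on.
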(event `ShowPauseMenu`
  (bind _returnvalue (`GameplayStatics.GetPlayerController` 0))
  (bind _returnvalue_2 (`|CreateWidget` "/Game/Night/UI_PauseMenu.UI_PauseMenu_C" _returnvalue))
  (set `self.PauseMenu` _returnvalue_2)
  (`UserWidget.AddToViewport` (`self.PauseMenu`) 0)
  (`WidgetBlueprintLibrary.SetInputMode_GameAndUIEx` _returnvalue (`self.PauseMenu`) "DoNotLock" false)
  (`GameplayStatics.SetGamePaused` true)
  (set `PlayerController.bShowMouseCursor` true _returnvalue))

(event `PauseMenuResume`
  (bind _returnvalue (`GameplayStatics.GetPlayerController` 0))
  (bind _foundwidgets (`WidgetBlueprintLibrary.GetAllWidgetsOfClass` "/Game/Night/UI_PauseMenu.UI_PauseMenu_C"))
  (`Widget.RemoveFromParent` _foundwidgets)
  (`GameplayStatics.SetGamePaused` false)
  (`WidgetBlueprintLibrary.SetInputMode_GameOnly` _returnvalue)
  (set `PlayerController.bShowMouseCursor` true _returnvalue))

(event `Key|P`
  (params (Key :type "Key Structure"))
  (:`Pressed`
    (`self.ShowPauseMenu`)))

(event `Key|U` :paused true
  (params (Key :type "Key Structure"))
  (:`Pressed`
    (`self.PauseMenuResume`)))