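; BPC_Sprinting is a character component that tracks the endurance spent on sprinting.
; Endurance starts at maximum, drains through OnSprint and refills through OnChill, clamped between zero and the maximum.
; Chill also updates RestEnd against a fixed threshold, so CanSprint blocks sprinting when endurance is empty or rest is unfinished.
; GetPercent exposes the remaining endurance as a fraction of the maximum.
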(event `self.ReceiveBeginPlay`
  (set `self.Endurance` (`self.Max Endurance`)))

(event `On Sprint`
  (params (`Sprint Amount` :type "Float (double-precision)"))
  (`self.Sprint` `Sprint Amount`))

(event `On Chill`
  (params (`Chill Amount` :type "Float (double-precision)"))
  (`self.Chill` `Chill Amount`))

(fn `Can Sprint`
  (returns (ReturnValue :type Boolean))
  (return (and (> (`self.Endurance`) 0.0) (`self.RestEnd`))))

(fn `Chill`
  (params (`Chill Amount` :type "Float (double-precision)"))
  (set `self.Endurance` (`KismetMathLibrary.FMin` (+ `Chill Amount` (`self.Endurance`)) (`self.Max Endurance`)))
  (`|ExecutionSequence`
    (:`then_1`
      (if (< (`self.Endurance`) 30.0)
        (set `self.RestEnd` false)))
    (:`then_2`
      (if (> (`self.Endurance`) 30.0)
        (set `self.RestEnd` true)))))

(fn `Get Percent`
  (returns (`Endurance Percent` :type "Float (double-precision)"))
  (return (/ (`self.Endurance`) (`self.Max Endurance`))))

(fn `Sprint`
  (params (`Sprint Amount` :type "Float (double-precision)"))
  (set `self.Endurance` (`KismetMathLibrary.FMax` (- (`self.Endurance`) `Sprint Amount`))))