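; Player hero character that walks, sprints, kicks small stones and carries data-table weapons.
; Tick picks run, walk or stand (while kicking) to set movement limits and feed the sprint component.
; BeginPlay creates the HUD, tints the health bar and attaches an overhead light; R triggers a delayed sphere-overlap kick that launches nearby stones.
; Kill strips weapons, ragdolls the mesh, then shows the death screen after a delay.
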(event `/Game/Night/BPI_Damageable.Kill`
  (bind _returnvalue (`self.K2_GetComponentsByClass` (`GameplayStatics.GetPlayerCharacter` 0) "/Game/Night/Weapons/BPC_Weapon.BPC_Weapon_C"))
  ;[0.2969 0.01561 0] Death
  (while (`KismetArrayLibrary.Array_IsNotEmpty` _returnvalue)
    (`ActorComponent.K2_DestroyComponent` _returnvalue))
  (`PrimitiveComponent.SetSimulatePhysics` (`self.Mesh`) true)
  (`PrimitiveComponent.SetCollisionEnabled` (`self.Mesh`) "PhysicsOnly")
  (`PrimitiveComponent.SetCollisionEnabled` (`self.CapsuleComponent`) "PhysicsOnly")
  (`self.K2_DestroyActor` (`/Game/Night/BPC_Damageable.Damageable Actor` (`self.BPC_Damageable`)))
  (`KismetSystemLibrary.Delay` 3.0)
  (`/Game/Night/UI/BPC_DeathScreen.ShowDeathScreen` (`self.BPC_DeathScreen`)))

(event `self.ReceiveBeginPlay`
  (bind _returnvalue (`self.GetTransform` self))
  (bind _asui_damageable_bar (cast `/Game/Night/UI/UI_Damageable_Bar` (`WidgetComponent.GetWidget` (`/Game/Night/BP_Damageable_Actor.Widget` (`/Game/Night/BPC_Damageable.Damageable Actor` (`self.BPC_Damageable`))))))
  (`ProgressBar.SetFillColorAndOpacity` (`/Game/Night/UI/UI_Damageable_Bar.HealthBar` _asui_damageable_bar) (struct :`G` 1.0 :`B` 0.207111 :`A` 1.0))
  (bind _returnvalue_2 (`|CreateWidget` "/Game/Night/UI/UI_HUD.UI_HUD_C"))
  (`UserWidget.AddToViewport` _returnvalue_2 0)
  (bind _returnvalue_3 (`|SpawnActorFromClass` "/Game/Night/Character/BP_LightSource.BP_LightSource_C" (`KismetMathLibrary.MakeTransform` (`KismetMathLibrary.MakeVector` (.x (.location _returnvalue)) (+ (.y (.location _returnvalue)) 100.0) (+ (.z (.location _returnvalue)) 300.0))) "Undefined" "OverrideRootScale" null null))
  (`self.K2_AttachToActor` _returnvalue_3 self "None" "KeepWorld" "KeepRelative" "KeepRelative" false))

(event `self.ReceiveTick`
  (params (DeltaSeconds :type "Float (single-precision)"))
  ;[1 1 1] Update Speed
  (`|ExecutionSequence`
    (:`then_0`
      (bind _should_run (`self.Should Run`))
      (if _should_run
        (`self.Run`)))
    (:`then_1`
      (bind _should_walk (`self.Should Walk`))
      (if _should_walk
        (`self.Walk`)))
    (:`then_2`
      (bind _should_stand (`self.Should Stand`))
      (if _should_stand
        (`self.Stand`)))))

(event `Key|R`
  (params (Key :type "Key Structure"))
  ;[1 1 1] Kick
  (:`Pressed`
    (if (not (`self.Is Kicking`))
      (set `self.Is Kicking` true)
      (`|ExecutionSequence`
        (:`then_0`
          (`KismetSystemLibrary.Delay` 0.7)
          (set `self.Is Kicking` false))
        (:`then_1`
          (`KismetSystemLibrary.Delay` 0.3)
          (`self.Kick`))))))

(fn `Add Weapon`
  (params (Tag :type String))
  (bind _returnvalue (`|GetDataTableRow` "/Game/Night/Weapons/DT_Weapons.DT_Weapons" (`KismetStringLibrary.Conv_StringToName` Tag))
    (:`then`
      (`|AddComponentByClass` (`.Component_9_D2EA33814F4A7972245013BF8146416B` (break `/Game/Night/Weapons/SK_Weapon` _returnvalue))))))

(fn `Kick`
  (bind _outactors (`KismetSystemLibrary.SphereOverlapActors` (`self.K2_GetActorLocation`) 100.0 (`|MakeArray` "ObjectTypeQuery2" :!type "EObjectTypeQuery Enum") "/Game/Night/LevelPrototyping/BP_Little_Stone.BP_Little_Stone_C"))
  (for _array_element _outactors
    (bind _asbp_little_stone (cast `/Game/Night/LevelPrototyping/BP_Little_Stone` _array_element))
    (`/Game/Night/LevelPrototyping/BP_Little_Stone.Kick` _asbp_little_stone (* (+ (`self.GetActorForwardVector`) (0.0 0.0 0.5)) 70000.0))))

(fn `Run`
  (set `CharacterMovementComponent.MaxAcceleration` (`self.Run Acceleration`) (`self.CharacterMovement`))
  (set `CharacterMovementComponent.MaxWalkSpeed` (`self.Run Speed`) (`self.CharacterMovement`))
  (`/Game/Night/Character/BPC_Sprinting.On Sprint` (`self.BPC_Sprinting`) 3.0))

(fn `Should Run`
  (returns (`Should Run` :type Boolean))
  (bind _should_stand (`self.Should Stand`))
  (if _should_stand
    (return false)
    (else
      (bind _returnvalue (`/Game/Night/Character/BPC_Sprinting.Can Sprint` (`self.BPC_Sprinting`)))
      (return (and _returnvalue (`|GetInputActionValue`))))))

(fn `Should Stand`
  (returns (`Should Stand` :type Boolean))
  (return (`self.Is Kicking`)))

(fn `Should Walk`
  (returns (`Should Walk` :type Boolean))
  (bind _should_run (`self.Should Run`))
  (if _should_run
    (return false)
    (else
      (bind _should_stand (`self.Should Stand`))
      (if _should_stand
        (return false)
        (else
          (return true))))))

(fn `Stand`
  (set `CharacterMovementComponent.MaxAcceleration` 0.0 (`self.CharacterMovement`))
  (set `CharacterMovementComponent.MaxWalkSpeed` 0.0 (`self.CharacterMovement`))
  (`/Game/Night/Character/BPC_Sprinting.On Chill` (`self.BPC_Sprinting`) 0.5))

(fn `UserConstructionScript`)

(fn `Walk`
  (set `CharacterMovementComponent.MaxAcceleration` (`self.Walk Acceleration`) (`self.CharacterMovement`))
  (set `CharacterMovementComponent.MaxWalkSpeed` (`self.Walk Speed`) (`self.CharacterMovement`))
  (`/Game/Night/Character/BPC_Sprinting.On Chill` (`self.BPC_Sprinting`) 0.5))