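; BPC_HeroExperience is a component that tracks experience and level for its owner, presumably the hero.
; On BeginPlay it spawns a BP_XP actor and attaches it to the owner.
; AddXP accumulates XP; at the threshold it raises the level, discards any overflow, scales the next threshold linearly with level, and prints debug values.
; GetLevelPercent returns progress toward the next level as a fraction.
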(event `self.ReceiveBeginPlay`
  (bind _returnvalue (`|SpawnActorFromClass` "/Game/Night/BP_XP.BP_XP_C" (`KismetMathLibrary.MakeTransform` (0.0 0.0 0.0)) "Undefined" "OverrideRootScale" null null))
  (`Actor.K2_AttachToActor` _returnvalue (`self.GetOwner`) "None" "KeepRelative" "KeepRelative" "KeepRelative" true))

(event `Add XP`
  (params (`XP+` :type "Float (double-precision)" :default 25.0))
  (set `self.CurrentXP` (+ `XP+` (`self.CurrentXP`)))
  (if (>= (`self.CurrentXP`) (`self.CurrentXPMax`))
    (`/Engine/EditorBlueprintResources/StandardMacros.IncrementInt` (`self.Level`)
      (:`  `
        (set `self.CurrentXP` 0.0)
        (set `self.CurrentXPMax` (`KismetMathLibrary.Conv_IntToDouble` (* (`self.Level`) 100)))
        (`KismetSystemLibrary.PrintString` (`KismetStringLibrary.Conv_IntToString` (`self.Level`)))
        (`KismetSystemLibrary.PrintString` (`KismetStringLibrary.Conv_DoubleToString` (`self.CurrentXP`)))))
    (else
      (`KismetSystemLibrary.PrintString` (`KismetStringLibrary.Conv_DoubleToString` (`self.CurrentXP`))))))

(fn `Get Level Percent`
  (returns (`Level Percent` :type "Float (double-precision)"))
  (return (/ (`self.CurrentXP`) (`self.CurrentXPMax`))))