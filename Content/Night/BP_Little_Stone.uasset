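; BP_Little_Stone is a kickable physics stone that kills enemies it passes near.
; Kick enables physics on the Stone component, applies an impulse and sets IsKicked.
; Tick moves the actor to the simulated Stone's location and calls Stop below a small speed threshold, clearing the flag and disabling physics.
; While kicked, a sphere overlap each tick calls Kill on nearby BP_Enemy pawns through BPI_Damageable.
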(event `self.ReceiveTick`
  (params (DeltaSeconds :type "Float (single-precision)"))
  (`|ExecutionSequence`
    (:`then_0`
      ;[1 1 1] Update position
      (`self.K2_SetActorLocation` (`SceneComponent.K2_GetComponentLocation` (`self.Stone`))))
    (:`then_1`
      ;[1 1 1] Update Velocity
      (bind _velocity (`self.Get Velocity`))
      (if (< _velocity 10.0)
        (`self.Stop`)))
    (:`then_2`
      ;[1 1 1] Kill enemies
      (if (`self.Is Kicked`)
        (bind _outactors (`KismetSystemLibrary.SphereOverlapActors` (`self.K2_GetActorLocation`) 75.0 (`|MakeArray` "ObjectTypeQuery3" :!type "EObjectTypeQuery Enum") "/Game/Night/Enemies/BP_Enemy.BP_Enemy_C"))
        (for _array_element _outactors
          (bind _asbpi_damageable (cast `/Game/Night/BPI_Damageable` _array_element))
          (`/Game/Night/BPI_Damageable.Kill` _asbpi_damageable))))))

(fn `Get Velocity`
  (returns (Velocity :type "Float (double-precision)"))
  (bind _returnvalue (`PrimitiveComponent.GetPhysicsLinearVelocity` (`self.Stone`) "None"))
  (return (`KismetMathLibrary.VSize` _returnvalue)))

(fn `Kick`
  (params (Direction :type "Vector Structure"))
  (`PrimitiveComponent.SetSimulatePhysics` (`self.Stone`) true)
  (`PrimitiveComponent.AddImpulse` (`self.Stone`) Direction "None" false)
  (set `self.Is Kicked` true))

(fn `Stop`
  (set `self.Is Kicked` false)
  (`PrimitiveComponent.SetSimulatePhysics` (`self.Stone`) false))

(fn `UserConstructionScript`)