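; Enemy character that hurts BP_Hero on contact and drops an experience sphere when killed.
; Capsule hits apply damage, throttled by a cooldown counted down in Tick.
; Walk speed is held constant by matching minimum analog speed to maximum on BeginPlay.
; Kill turns on mesh physics, destroys the damageable component's linked actor, then later disables mesh collision responses and expires the body through its lifespan.
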(event `self.ReceiveBeginPlay`
  ;[0.6217 0.3875 0.9052] Common Setup / Initialization
  (`|ExecutionSequence`
    (:`then_0`
      (`self.Set Const Move Speed` (`self.Base Move Speed`)))))

(event `/Game/Night/BPI_Damageable.Kill`
  ;[0.8844 0.4582 0.2644] Death
  (`|SpawnActorFromClass` "/Game/Night/BP_ExperienceSphere.BP_ExperienceSphere_C" (`self.GetTransform` self) "Undefined" "OverrideRootScale" null null)
  (`PrimitiveComponent.SetSimulatePhysics` (`self.Mesh`) true)
  (`PrimitiveComponent.SetCollisionEnabled` (`self.Mesh`) "PhysicsOnly")
  (`PrimitiveComponent.SetCollisionEnabled` (`self.CapsuleComponent`) "PhysicsOnly")
  (`self.K2_DestroyActor` (`/Game/Night/BPC_Damageable.Damageable Actor` (`self.BPC_Damageable`)))
  (`KismetSystemLibrary.Delay` 10.0)
  (`PrimitiveComponent.SetCollisionResponseToAllChannels` (`self.Mesh`) "ECR_Ignore")
  (`self.SetLifeSpan` 5.0))

(event `self.CapsuleComponent.OnComponentHit`
  (params (HitComponent :type "PrimitiveComponent Object Reference") (OtherActor :type "Actor Object Reference") (OtherComp :type "PrimitiveComponent Object Reference") (NormalImpulse :type "Vector Structure") (Hit :type "HitResult Structure (by ref)"))
  ;[0.136 0.8927 0.2749] Contact Damage
  (if (<= (`self.Cooldown`) 0.0)
    (bind _asbp_hero (cast `/Game/Night/BP_Hero` OtherActor))
    (`GameplayStatics.ApplyDamage` _asbp_hero (`self.Damage`))
    (set `self.Cooldown` (`self.Cooldown Max`))))

(event `self.ReceiveTick`
  (params (DeltaSeconds :type "Float (single-precision)"))
  ;[0.136 0.8927 0.2749] Contact Damage
  (set `self.Cooldown` (- (`self.Cooldown`) DeltaSeconds)))

(fn `Set Const Move Speed`
  (params (`Move Speed` :type "Float (double-precision)"))
  (bind _charactermovement (`self.CharacterMovement`))
  (bind _output_get (set `CharacterMovementComponent.MaxWalkSpeed` `Move Speed` _charactermovement))
  (set `CharacterMovementComponent.MinAnalogWalkSpeed` _output_get _charactermovement))

(fn `UserConstructionScript`)