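; Night enemy Blueprint that repeatedly charges in a straight line toward the player's position.
; A Tick-driven state machine cycles through Idle, Preparing and Ramming after running the parent Tick.
; Preparing captures the direction to player 0 in a single tick, so the charge does not home in.
; Ramming applies movement input along that direction for a set time, then Idle counts down before the next charge.
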(event `self.ReceiveTick`
  (params (DeltaSeconds :type "Float (single-precision)"))
  (`parent.ReceiveTick` DeltaSeconds)
  (switch `/Game/Night/Enemies/E_RamState` (`self.Ram State`)
    (:`NewEnumerator0`
      ;[0.7094 0.1501 0.1967] Idle
      (if (> (`self.Rem Idle Time`) 0.0)
        (set `self.Rem Idle Time` (- (`self.Rem Idle Time`) (`GameplayStatics.GetWorldDeltaSeconds`)))
        (else
          (set `self.Ram State` "NewEnumerator1"))))
    (:`NewEnumerator1`
      ;[0.876 0.6723 0.1706] Preparing
      (set `self.Ram Dir` (- (`self.K2_GetActorLocation` (`GameplayStatics.GetPlayerCharacter` 0)) (`self.K2_GetActorLocation`)))
      (set `self.Rem Ram Time` (`self.Ram Seconds`))
      (set `self.Ram State` "NewEnumerator2"))
    (:`NewEnumerator2`
      ;[0.1258 0.976 0.2834] Ramming
      (if (> (`self.Rem Ram Time`) 0.0)
        (`self.AddMovementInput` (`self.Ram Dir`))
        (set `self.Rem Ram Time` (- (`self.Rem Ram Time`) (`GameplayStatics.GetWorldDeltaSeconds`)))
        (else
          (set `self.Ram Dir` (0.0 0.0 0.0))
          (set `self.Rem Idle Time` (`self.Prepare Seconds`))
          (set `self.Ram State` "NewEnumerator0"))))))

(fn `UserConstructionScript`
  (`parent.UserConstructionScript`))