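; Actor component that periodically spawns simple chasing enemies around the hero in the night enemy set.
; Tick accumulates elapsed time and, whenever it passes a threshold that advances by one second, spawns an enemy relative to the hero's transform.
; A random X offset and a square-root Y offset with random sign aim to place spawns on a ring around the hero, at the hero's height and rotation.
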(event `self.ReceiveTick`
  (params (DeltaSeconds :type "Float (single-precision)"))
  (bind _returnvalue (`KismetMathLibrary.RandomFloatInRange` -2000.0 2000.0))
  (bind _output_get (set `self.Time` (+ (`self.Time`) (`GameplayStatics.GetWorldDeltaSeconds`))))
  (if (> _output_get (`self.SpawnTime`))
    (set `self.SpawnTime` (+ (`self.SpawnTime`) 1.0))
    (bind _returnvalue_2 (`GameplayStatics.GetActorOfClass` "/Game/Night/Character/BP_Hero.BP_Hero_C"))
    (bind _returnvalue_3 (`Actor.GetTransform` _returnvalue_2))
    (bind _returnvalue_4 (`|SpawnActorFromClass` "/Game/Night/Enemies/BP_Enemy_SimpleChasing.BP_Enemy_SimpleChasing_C" (`KismetMathLibrary.MakeTransform` (`KismetMathLibrary.MakeVector` (+ _returnvalue (.x (.location _returnvalue_3))) (+ (.y (.location _returnvalue_3)) (* (`KismetArrayLibrary.Array_Random` (`self.OneAndMinusOne`)) (`KismetMathLibrary.Sqrt` (- 4000000.0 (`KismetMathLibrary.Square` _returnvalue))))) (.z (.location _returnvalue_3))) (.rotation _returnvalue_3)) "Undefined" "OverrideRootScale" null null))))