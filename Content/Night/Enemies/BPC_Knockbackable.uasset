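; Actor component that lets an enemy character be knocked back, scaled by a knockback resistance setting.
; On BeginPlay it converts the resistance percentage into a power multiplier and caches the owner as a Character.
; KnockBack launches that character with the given vector times the multiplier, adding to its current velocity rather than overriding it.
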(event `self.ReceiveBeginPlay`
  (`|ExecutionSequence`
    (:`then_0`
      (set `self.KB Power Mult` (- 1.0 (/ (`self.Knockback Resistence %`) 100.0))))
    (:`then_1`
      (bind _ascharacter (cast `Character` (`self.GetOwner`)))
      (set `self.Owner Char` _ascharacter))))

(fn `Knock Back`
  (params (`Knockback Vec` :type "Vector Structure"))
  (`Character.LaunchCharacter` (`self.Owner Char`) (* `Knockback Vec` (`self.KB Power Mult`)) false false))