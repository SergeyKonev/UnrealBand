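; BP_LevelPart is a level tile that grows the world endlessly around BP_Hero.
; On construction it registers its location with BP_Level.
; When the hero overlaps its Trigger, it destroys the trigger and runs eight directional spawn functions, one per neighbour.
; Each offsets from the actor bounds by twice the extent and spawns another BP_LevelPart only if BP_Level's CheckLevelPart returns false for that spot.
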(event `self.Trigger.OnComponentBeginOverlap`
  (params (OverlappedComponent :type "PrimitiveComponent Object Reference") (OtherActor :type "Actor Object Reference") (OtherComp :type "PrimitiveComponent Object Reference") (OtherBodyIndex :type Integer) (bFromSweep :type Boolean) (SweepResult :type "HitResult Structure (by ref)"))
  (cast `/Game/Night/BP_Hero` OtherActor)
  (`ActorComponent.K2_DestroyComponent` (`self.Trigger`))
  (`self.SpawnLeft`)
  (`self.SpawUpLeft`)
  (`self.SpawnUp`)
  (`self.SpawnUpRight`)
  (`self.SpawnRight`)
  (`self.SpawnDownRight`)
  (`self.SpawnDown`)
  (`self.SpawnDownLeft`))

(fn `SpawnDown`
  (bind (_origin _boxextent) (`self.GetActorBounds` self false false))
  (bind _returnvalue (- (.x _origin) (* (.x _boxextent) 2.0)))
  (bind _returnvalue_2 (`GameplayStatics.GetActorOfClass` "/Game/Night/BP_Level.BP_Level_C"))
  (bind _newparam1 (`/Game/Night/BP_Level.CheckLevelPart` _returnvalue_2 (`KismetMathLibrary.MakeVector` _returnvalue (.y _origin) (.z _origin))))
  (if (not _newparam1)
    (`|SpawnActorFromClass` "BP_LevelPart_C" (`KismetMathLibrary.MakeTransform` (`KismetMathLibrary.MakeVector` _returnvalue (.y _origin) (.z _origin))) "AlwaysSpawn" "OverrideRootScale" null null)))

(fn `SpawnDownLeft`
  (bind (_origin _boxextent) (`self.GetActorBounds` self false false))
  (bind _returnvalue (- (.y _origin) (* (.y _boxextent) 2.0)))
  (bind _returnvalue_2 (- (.x _origin) (* (.x _boxextent) 2.0)))
  (bind _returnvalue_3 (`GameplayStatics.GetActorOfClass` "/Game/Night/BP_Level.BP_Level_C"))
  (bind _newparam1 (`/Game/Night/BP_Level.CheckLevelPart` _returnvalue_3 (`KismetMathLibrary.MakeVector` _returnvalue_2 _returnvalue (.z _origin))))
  (if (not _newparam1)
    (`|SpawnActorFromClass` "BP_LevelPart_C" (`KismetMathLibrary.MakeTransform` (`KismetMathLibrary.MakeVector` _returnvalue_2 _returnvalue (.z _origin))) "AlwaysSpawn" "OverrideRootScale" null null)))

(fn `SpawnDownRight`
  (bind (_origin _boxextent) (`self.GetActorBounds` self false false))
  (bind _returnvalue (- (.x _origin) (* (.x _boxextent) 2.0)))
  (bind _returnvalue_2 (+ (.y _origin) (* (.y _boxextent) 2.0)))
  (bind _returnvalue_3 (`GameplayStatics.GetActorOfClass` "/Game/Night/BP_Level.BP_Level_C"))
  (bind _newparam1 (`/Game/Night/BP_Level.CheckLevelPart` _returnvalue_3 (`KismetMathLibrary.MakeVector` _returnvalue _returnvalue_2 (.z _origin))))
  (if (not _newparam1)
    (`|SpawnActorFromClass` "BP_LevelPart_C" (`KismetMathLibrary.MakeTransform` (`KismetMathLibrary.MakeVector` _returnvalue _returnvalue_2 (.z _origin))) "AlwaysSpawn" "OverrideRootScale" null null)))

(fn `SpawnLeft`
  (bind (_origin _boxextent) (`self.GetActorBounds` self false false))
  (bind _returnvalue (- (.y _origin) (* (.y _boxextent) 2.0)))
  (bind _returnvalue_2 (`GameplayStatics.GetActorOfClass` "/Game/Night/BP_Level.BP_Level_C"))
  (bind _newparam1 (`/Game/Night/BP_Level.CheckLevelPart` _returnvalue_2 (`KismetMathLibrary.MakeVector` (.x _origin) _returnvalue (.z _origin))))
  (if (not _newparam1)
    (`|SpawnActorFromClass` "BP_LevelPart_C" (`KismetMathLibrary.MakeTransform` (`KismetMathLibrary.MakeVector` (.x _origin) _returnvalue (.z _origin))) "AlwaysSpawn" "OverrideRootScale" null null)))

(fn `SpawnRight`
  (bind (_origin _boxextent) (`self.GetActorBounds` self false false))
  (bind _returnvalue (+ (.y _origin) (* (.y _boxextent) 2.0)))
  (bind _returnvalue_2 (`GameplayStatics.GetActorOfClass` "/Game/Night/BP_Level.BP_Level_C"))
  (bind _newparam1 (`/Game/Night/BP_Level.CheckLevelPart` _returnvalue_2 (`KismetMathLibrary.MakeVector` (.x _origin) _returnvalue (.z _origin))))
  (if (not _newparam1)
    (`|SpawnActorFromClass` "BP_LevelPart_C" (`KismetMathLibrary.MakeTransform` (`KismetMathLibrary.MakeVector` (.x _origin) _returnvalue (.z _origin))) "AlwaysSpawn" "OverrideRootScale" null null)))

(fn `SpawnUp`
  (bind (_origin _boxextent) (`self.GetActorBounds` self false false))
  (bind _returnvalue (+ (.x _origin) (* (.x _boxextent) 2.0)))
  (bind _returnvalue_2 (`GameplayStatics.GetActorOfClass` "/Game/Night/BP_Level.BP_Level_C"))
  (bind _newparam1 (`/Game/Night/BP_Level.CheckLevelPart` _returnvalue_2 (`KismetMathLibrary.MakeVector` _returnvalue (.y _origin) (.z _origin))))
  (if (not _newparam1)
    (`|SpawnActorFromClass` "BP_LevelPart_C" (`KismetMathLibrary.MakeTransform` (`KismetMathLibrary.MakeVector` _returnvalue (.y _origin) (.z _origin))) "AlwaysSpawn" "OverrideRootScale" null null)))

(fn `SpawnUpRight`
  (bind (_origin _boxextent) (`self.GetActorBounds` self false false))
  (bind _returnvalue (+ (.x _origin) (* (.x _boxextent) 2.0)))
  (bind _returnvalue_2 (+ (.y _origin) (* (.y _boxextent) 2.0)))
  (bind _returnvalue_3 (`GameplayStatics.GetActorOfClass` "/Game/Night/BP_Level.BP_Level_C"))
  (bind _newparam1 (`/Game/Night/BP_Level.CheckLevelPart` _returnvalue_3 (`KismetMathLibrary.MakeVector` _returnvalue _returnvalue_2 (.z _origin))))
  (if (not _newparam1)
    (`|SpawnActorFromClass` "BP_LevelPart_C" (`KismetMathLibrary.MakeTransform` (`KismetMathLibrary.MakeVector` _returnvalue _returnvalue_2 (.z _origin))) "AlwaysSpawn" "OverrideRootScale" null null)))

(fn `SpawUpLeft`
  (bind (_origin _boxextent) (`self.GetActorBounds` self false false))
  (bind _returnvalue (- (.y _origin) (* (.y _boxextent) 2.0)))
  (bind _returnvalue_2 (+ (.x _origin) (* (.x _boxextent) 2.0)))
  (bind _returnvalue_3 (`GameplayStatics.GetActorOfClass` "/Game/Night/BP_Level.BP_Level_C"))
  (bind _newparam1 (`/Game/Night/BP_Level.CheckLevelPart` _returnvalue_3 (`KismetMathLibrary.MakeVector` _returnvalue_2 _returnvalue (.z _origin))))
  (if (not _newparam1)
    (`|SpawnActorFromClass` "BP_LevelPart_C" (`KismetMathLibrary.MakeTransform` (`KismetMathLibrary.MakeVector` _returnvalue_2 _returnvalue (.z _origin))) "AlwaysSpawn" "OverrideRootScale" null null)))

(fn `UserConstructionScript`
  (bind _returnvalue_location (`KismetMathLibrary.BreakTransform` (`self.GetTransform`)))
  (bind _returnvalue (`GameplayStatics.GetActorOfClass` "/Game/Night/BP_Level.BP_Level_C"))
  (`/Game/Night/BP_Level.AddLevelPart` _returnvalue _returnvalue_location))