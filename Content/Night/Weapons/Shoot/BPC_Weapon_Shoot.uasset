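; Weapon component for projectile attacks that fires one bullet from its owner each time Attack runs.
; Attack extends the parent weapon's logic, then builds a spawn transform from the Aiming mode: the owner's forward transform, or a look-at toward a random or nearest enemy.
; It spawns BulletClass at that transform, passing the Pierce value and itself as the bullet's Weapon.
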(fn `Attack`
  (locals (`Local Transform` :type "Transform Structure"))
  (bind _returnvalue (`Actor.K2_GetActorLocation` (`self.GetOwner`)))
  (bind _returnvalue_2 (`Actor.K2_GetActorLocation` (`self.GetOwner`)))
  (`parent.Attack`)
  (`|ExecutionSequence`
    (:`then_0`
      (set `local.Local Transform` (select `/Game/Night/Weapons/E_Aiming` (`self.Aiming`) :`NewEnumerator0` (`Actor.GetTransform` (`self.GetOwner`)) :`NewEnumerator1` (`KismetMathLibrary.MakeTransform` _returnvalue_2 (`KismetMathLibrary.FindLookAtRotation` _returnvalue_2 (`Actor.K2_GetActorLocation` (`self.Get Random Enemy`)))) :`NewEnumerator2` (`KismetMathLibrary.MakeTransform` _returnvalue (`KismetMathLibrary.FindLookAtRotation` _returnvalue (`Actor.K2_GetActorLocation` (`self.Get Nearest Enemy` _returnvalue)))))))
    (:`then_1`
      (`|SpawnActorFromClass` (`self.Bullet Class`) (`local.Local Transform`) "Undefined" "OverrideRootScale" null (`self.Pierce`) self null))))