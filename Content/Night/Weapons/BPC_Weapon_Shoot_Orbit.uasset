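; Weapon component that gives the player an orbit weapon by ensuring a BP_Orbit actor exists in the level.
; On BeginPlay, after the parent logic, it looks for a BP_Orbit and, if none exists, spawns one at the player character's transform.
; The new orbit is stored in MyOrbit and attached to the player; an existing one is left untouched and not stored.
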(event `self.ReceiveBeginPlay`
  (`parent.ReceiveBeginPlay`)
  (bind _returnvalue (`GameplayStatics.GetActorOfClass` "/Game/Night/Weapons/BP_Orbit.BP_Orbit_C"))
  (if (not (`KismetSystemLibrary.IsValid` _returnvalue))
    (bind _returnvalue_2 (`|SpawnActorFromClass` "/Game/Night/Weapons/BP_Orbit.BP_Orbit_C" (`Actor.GetTransform` (`GameplayStatics.GetPlayerCharacter` 0)) "Undefined" "OverrideRootScale" null null))
    (set `self.My Orbit` _returnvalue_2)
    (`Actor.K2_AttachToActor` _returnvalue_2 (`GameplayStatics.GetPlayerCharacter` 0) "None" "KeepWorld" "KeepRelative" "KeepRelative" true)))