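; BPC_Weapon is a base weapon component that fires automatically on a repeating cooldown.
; Tick counts Cooldown down, then resets it to CooldownMax and calls Attack, which is empty here.
; DamageEnemy applies Damage through the enemy's damageable component and a 2D knockback away from the owner through its knockbackable component.
; Targeting helpers return the nearest or a random BP_Enemy by searching all actors of that class.
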(event `self.ReceiveTick`
  (params (DeltaSeconds :type "Float (single-precision)"))
  (if (> (`self.Cooldown`) 0.0)
    (set `self.Cooldown` (- (`self.Cooldown`) (`GameplayStatics.GetWorldDeltaSeconds`)))
    (else
      (set `self.Cooldown` (`self.Cooldown Max`))
      (`self.Attack`))))

(fn `Attack`)

(fn `Damage Enemy`
  (params (Enemy :type "/Game/Night/Enemies/BP_Enemy Object Reference"))
  (`/Game/Night/BPC_Damageable.Hurt` (`/Game/Night/Enemies/BP_Enemy.BPC_Damageable` Enemy) (`self.Damage`))
  (`/Game/Night/Enemies/BPC_Knockbackable.Knock Back` (`/Game/Night/Enemies/BP_Enemy.BPC_Knockbackable` Enemy) (* (`KismetMathLibrary.Normal` (- (`KismetMathLibrary.Conv_VectorToVector2D` (`Actor.K2_GetActorLocation` Enemy)) (`KismetMathLibrary.Conv_VectorToVector2D` (`Actor.K2_GetActorLocation` (`self.GetOwner`))))) (`self.Knockback`))))

(fn `Get Nearest Enemy`
  (params (`In Location` :type "Vector Structure"))
  (returns (Enemy :type "/Game/Night/Enemies/BP_Enemy Object Reference"))
  (bind _outactors (`GameplayStatics.GetAllActorsOfClass` "/Game/Night/Enemies/BP_Enemy.BP_Enemy_C"))
  (bind _asbp_enemy (cast `/Game/Night/Enemies/BP_Enemy` (`.ReturnValue` (`GameplayStatics.FindNearestActor` `In Location` _outactors))))
  (return _asbp_enemy))

(fn `Get Random Enemy`
  (returns (Enemy :type "/Game/Night/Enemies/BP_Enemy Object Reference"))
  (bind _outactors (`GameplayStatics.GetAllActorsOfClass` "/Game/Night/Enemies/BP_Enemy.BP_Enemy_C"))
  (return (`KismetArrayLibrary.Array_Random` _outactors)))